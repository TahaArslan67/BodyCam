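; BodyCam_BP is a body camera pickup that changes the first-person character's view.
; A capsule overlap stores the BP_FirstPersonCharacter and sets an in-area flag, which is never cleared.
; Tick then polls the character's EBasildi (E pressed) flag.
; When that flag is set, the actor destroys itself, lowers the character's FirstPersonCamera and adds a PostProcess component to the character.
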(event OnComponentBeginOverlap(Capsule)
  (params (OverlappedComponent :type Primitive%20Component%20Object%20Reference) (OtherActor :type Actor%20Object%20Reference) (OtherComp :type Primitive%20Component%20Object%20Reference) (OtherBodyIndex :type Integer) (bFromSweep :type Boolean) (SweepResult :type Hit%20Result%20Structure%20%28by%20ref%29))
  (bind _asbp_first_person_character (Utilities|Casting|CastToBP_FirstPersonCharacter OtherActor))
  (Variables|Default|SetAlanaGirildimi true))

(event EventTick
  (params (DeltaSeconds :type Float%20%28single-precision%29))
  (if (Variables|Default|GetAlanaGirildimi)
    (if (Variables|/Game/FirstPerson/Blueprints/BP_FirstPersonCharacter.BP_FirstPersonCharacter_C|GetE%20basildi (stale OnComponentBeginOverlap(Capsule) _asbp_first_person_character))
      (Actor|DestroyActor)
      (Transformation|SetRelativeLocation (Variables|/Game/FirstPerson/Blueprints/BP_FirstPersonCharacter.BP_FirstPersonCharacter_C|GetFirstPersonCamera (stale OnComponentBeginOverlap(Capsule) _asbp_first_person_character)) (- (Variables|/Script/Engine.SceneComponent|GetRelativeLocation (Variables|/Game/FirstPerson/Blueprints/BP_FirstPersonCharacter.BP_FirstPersonCharacter_C|GetFirstPersonCamera (stale OnComponentBeginOverlap(Capsule) _asbp_first_person_character))) "0.000000,0.000000,15.000000") true false)
      (AddComponent|AddPostProcessComponent (stale OnComponentBeginOverlap(Capsule) _asbp_first_person_character) false))))

(fn ConstructionScript)